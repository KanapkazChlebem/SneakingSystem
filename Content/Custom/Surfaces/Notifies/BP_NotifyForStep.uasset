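; Animation notify for footsteps that plays a surface-specific step sound and makes the player's steps audible to AI.
; It line-traces from the mesh owner's location along its up vector by TraceLength and switches on the hit's physical surface.
; Grass, concrete and wood each have their own sound and noise range, with concrete as the fallback.
; The noise event is reported only when the owner is the player character.
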(fn ReceivedNotify
  (params (MeshComp :type Skeletal%20Mesh%20Component%20Object%20Reference) (Animation :type Anim%20Sequence%20Base%20Object%20Reference) (EventReference :type Anim%20Notify%20Event%20Reference%20Structure%20%28by%20ref%29))
  (CallFunction|HandleSound MeshComp 1.0)
  (return false))

(fn HandleSound
  (params (actor :type Actor%20Component%20Object%20Reference) (volumeMultiplier :type Float%20%28double-precision%29))
  (bind _returnvalue (Components|GetOwner actor))
  (bind _returnvalue_2 (Transformation|GetActorLocation _returnvalue))
  (bind _output_get (LocalVariables|SetactorLocation _returnvalue_2))
  (bind _outhit (Collision|LineTraceByChannel _output_get (+ _returnvalue_2 (* (Transformation|GetActorUpVector _returnvalue) (Variables|Default|GetTrace%20Length))) "TraceTypeQuery1" false 0 "ForDuration"))
  (switch Utilities|FlowControl|Switch|SwitchonEPhysicalSurface (Collision|GetSurfaceType _outhit)
    (:SurfaceType_Default
      ;[1 1 1] Default step sound
      (Audio|PlaySoundatLocation "/Game/Custom/Sounds/SoundCue/SC_ConcreteStep.SC_ConcreteStep" (LocalVariables|GetactorLocation) "0, 0, 0" volumeMultiplier 0.8 0.0 0 0 0 0)
      (CallFunction|ReportNoiseOfPlayerwithRange actor (Variables|Default|GetConcreteStepRange)))
    (:SurfaceType1
      ;[1 1 1] Grass step sound
      (Audio|PlaySoundatLocation "/Game/Custom/Sounds/SoundCue/SC_GrassStep.SC_GrassStep" (LocalVariables|GetactorLocation) "0, 0, 0" volumeMultiplier 1.0 0.0 0 0 0 0)
      (CallFunction|ReportNoiseOfPlayerwithRange actor (Variables|Default|GetGrassStepRange)))
    (:SurfaceType2
      ;[1 1 1] Concrete step sound
      (Audio|PlaySoundatLocation "/Game/Custom/Sounds/SoundCue/SC_ConcreteStep.SC_ConcreteStep" (LocalVariables|GetactorLocation) "0, 0, 0" volumeMultiplier 0.8 0.0 0 0 0 0)
      (CallFunction|ReportNoiseOfPlayerwithRange actor (Variables|Default|GetConcreteStepRange)))
    (:SurfaceType3
      ;[1 1 1] Wood step sound
      (Audio|PlaySoundatLocation "/Game/Custom/Sounds/SoundCue/SC_WoodStep.SC_WoodStep" (LocalVariables|GetactorLocation) "0, 0, 0" volumeMultiplier 1.0 0.0 0 0 0 0)
      (CallFunction|ReportNoiseOfPlayerwithRange actor (Variables|Default|GetWoodStepRange)))))

(fn ReportNoiseOfPlayerwithRange
  (params (actor :type Actor%20Component%20Object%20Reference) (range :type Float%20%28double-precision%29))
  (bind _returnvalue (Components|GetOwner actor))
  (if (== (Game|GetPlayerCharacter 0) _returnvalue)
    (Class|AISenseHearing|ReportNoiseEvent (Transformation|GetActorLocation _returnvalue) 1.0 _returnvalue range "None")))