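; Hiding spot volume that hides the player while they crouch inside it.
; It extends parent collision enter/leave handling, hiding an already crouched player on a successful entry and unhiding on a successful exit.
; Crouch and stand-up events also toggle hiding.
; Hide and Unhide pass the volume itself as a message to the player's sneaking component.
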(event EventBeginPlay
  (|CallParentFunction) ; This node is disabled and will not be called.\nDrag off pins to build functionality.
)

(event Collision|EventActorBeginOverlap
  (params (OtherActor :type Actor%20Object%20Reference))
  (|CallParentFunction OtherActor) ; This node is disabled and will not be called.\nDrag off pins to build functionality.
)

(event EventTick
  (params (DeltaSeconds :type Float%20%28single-precision%29))
  (|CallParentFunction DeltaSeconds) ; This node is disabled and will not be called.\nDrag off pins to build functionality.
)

(event EventPlayerStoodUp
  (CallFunction|Unhide))

(event EventPlayerCrouched
  (CallFunction|Hide))

(fn ConstructionScript
  (|CallParentFunction))

(fn PlayerEnterCollision
  (params (A :type Object%20Object%20Reference))
  (bind _isplayer (|CallParentFunction A))
  (if _isplayer
    (if (AI|Components|NavMovement|IsCrouching (Variables|/Script/Engine.Character|GetCharacterMovement (Variables|Default|GetplayerCharacterRef)))
      (CallFunction|Hide))))

(fn PlayerLeaveCollision
  (params (A :type Object%20Object%20Reference))
  (bind _isplayer (|CallParentFunction A))
  (if _isplayer
    (CallFunction|Unhide)))

(fn Unhide
  (Class|BPISneaking|Unhide(Message) (Variables|Default|GetplayerCharacterSneakingCompRef) self))

(fn Hide
  (Class|BPISneaking|Hide(Message) (Variables|Default|GetplayerCharacterSneakingCompRef) self))