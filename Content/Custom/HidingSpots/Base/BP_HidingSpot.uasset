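; BP_HidingSpot is a base hiding-spot actor with a Box trigger for detecting when the player enters or leaves.
; On BeginPlay it caches the player character and its BP_CharacterSneakingComponent.
; Box overlap events pass the other actor to PlayerEnterCollision and PlayerLeaveCollision, which only return whether it is the player.
; The sneaking component is not used here, and the overlap events ignore those results.
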(event OnComponentBeginOverlap(Box)
  (params (OverlappedComponent :type Primitive%20Component%20Object%20Reference) (OtherActor :type Actor%20Object%20Reference) (OtherComp :type Primitive%20Component%20Object%20Reference) (OtherBodyIndex :type Integer) (bFromSweep :type Boolean) (SweepResult :type Hit%20Result%20Structure%20%28by%20ref%29))
  (CallFunction|PlayerEnterCollision OtherActor))

(event OnComponentEndOverlap(Box)
  (params (OverlappedComponent :type Primitive%20Component%20Object%20Reference) (OtherActor :type Actor%20Object%20Reference) (OtherComp :type Primitive%20Component%20Object%20Reference) (OtherBodyIndex :type Integer))
  (CallFunction|PlayerLeaveCollision OtherActor))

(event EventBeginPlay
  (bind _output_get (Variables|Default|SetplayerCharacterRef (Game|GetPlayerCharacter 0)))
  (Variables|Default|SetplayerCharacterSneakingCompRef (Actor|GetComponentbyClass _output_get "/Game/Custom/Character/BP_CharacterSneakingComponent.BP_CharacterSneakingComponent_C")))

(event Collision|EventActorBeginOverlap
  (params (OtherActor :type Actor%20Object%20Reference)))

(event EventTick
  (params (DeltaSeconds :type Float%20%28single-precision%29)))

(fn ConstructionScript)

(fn PlayerEnterCollision
  (params (A :type Object%20Object%20Reference))
  (return (== A (Variables|Default|GetplayerCharacterRef))))

(fn PlayerLeaveCollision
  (params (A :type Object%20Object%20Reference))
  (return (== A (Variables|Default|GetplayerCharacterRef))))