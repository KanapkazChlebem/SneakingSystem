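; BP_TrashCan is a trash can hiding spot the player can interact with.
; Box overlap by the player shows an interaction prompt, which is removed on exit unless the player is hiding inside.
; Interact toggles the IsPlayerIn flag and shows or hides a stand-in PlayerModel, without itself moving or possessing the character.
; AddYaw rotates the can's SpringArm by the supplied yaw.
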(event OnComponentBeginOverlap(Box)
  (params (OverlappedComponent :type Primitive%20Component%20Object%20Reference) (OtherActor :type Actor%20Object%20Reference) (OtherComp :type Primitive%20Component%20Object%20Reference) (OtherBodyIndex :type Integer) (bFromSweep :type Boolean) (SweepResult :type Hit%20Result%20Structure%20%28by%20ref%29))
  (if (== OtherActor (Variables|Default|GetplayerCharacterRef))
    (UserInterface|Viewport|AddtoViewport (Variables|Default|GetinteractionWidget) 0)))

(event OnComponentEndOverlap(Box)
  (params (OverlappedComponent :type Primitive%20Component%20Object%20Reference) (OtherActor :type Actor%20Object%20Reference) (OtherComp :type Primitive%20Component%20Object%20Reference) (OtherBodyIndex :type Integer))
  (if (== OtherActor (Variables|Default|GetplayerCharacterRef))
    (if (not (Variables|Default|GetisPlayerIn))
      (Widget|RemovefromParent (Variables|Default|GetinteractionWidget)))))

(event EventBeginPlay
  (Variables|Default|SetplayerControllerRef (Game|GetPlayerController 0))
  (Variables|Default|SetplayerCharacterRef (Game|GetPlayerCharacter 0))
  (bind _returnvalue (UserInterface|CreateWidget "/Game/Custom/HUD/BPWidgetPrompt_Interaction.BPWidgetPrompt_Interaction_C"))
  (Variables|Default|SetinteractionWidget _returnvalue))

(event Collision|EventActorBeginOverlap
  (params (OtherActor :type Actor%20Object%20Reference)))

(event EventTick
  (params (DeltaSeconds :type Float%20%28single-precision%29)))

(event EventInteract
  (if (Variables|Default|GetisPlayerIn)
    (Variables|Default|SetisPlayerIn false)
    (Rendering|SetVisibility (Variables|Default|GetPlayerModel) false false)
    (else
      (Variables|Default|SetisPlayerIn true)
      (Rendering|SetVisibility (Variables|Default|GetPlayerModel) true false))))

(event EventAddYaw
  (params (yaw :type Float%20%28double-precision%29))
  (Transformation|AddRelativeRotation (Variables|Default|GetSpringArm) (Math|Rotator|MakeRotator 0.0 0.0 yaw) false false))

(fn ConstructionScript)