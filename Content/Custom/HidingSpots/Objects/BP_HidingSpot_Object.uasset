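; BP_HidingSpot_Object is a hiding spot object that the player can interact with to enter or leave.
; It creates an interaction prompt widget on BeginPlay, showing or removing it when the parent's collision enter and leave checks pass.
; Interact toggles the IsPlayerIn flag and shows the PlayerModel while occupied.
; AddYaw rotates the SpringArm horizontally by the supplied yaw.
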(event EventBeginPlay
  (|CallParentFunction)
  (bind _returnvalue (UserInterface|CreateWidget "/Game/Custom/HUD/BPWidgetPrompt_Interaction.BPWidgetPrompt_Interaction_C"))
  (Variables|Default|SetInteractionWidget _returnvalue))

(event Collision|EventActorBeginOverlap
  (params (OtherActor :type Actor%20Object%20Reference))
  (|CallParentFunction OtherActor) ; This node is disabled and will not be called.\nDrag off pins to build functionality.
)

(event EventTick
  (params (DeltaSeconds :type Float%20%28single-precision%29))
  (|CallParentFunction DeltaSeconds) ; This node is disabled and will not be called.\nDrag off pins to build functionality.
)

(event EventInteract
  (if (Variables|Default|GetisPlayerIn)
    (Variables|Default|SetisPlayerIn false)
    (Rendering|SetVisibility (Variables|Default|GetPlayerModel) false false)
    (else
      (Variables|Default|SetisPlayerIn true)
      (Rendering|SetVisibility (Variables|Default|GetPlayerModel) true false))))

(event EventAddYaw
  (params (yaw :type Float%20%28double-precision%29))
  (Transformation|AddRelativeRotation (Variables|Default|GetSpringArm) (Math|Rotator|MakeRotator 0.0 0.0 yaw) false false))

(fn ConstructionScript
  (|CallParentFunction))

(fn PlayerEnterCollision
  (params (A :type Object%20Object%20Reference))
  (bind _isplayer (|CallParentFunction A))
  (if _isplayer
    (UserInterface|Viewport|AddtoViewport (Variables|Default|GetInteractionWidget) 0)))

(fn PlayerLeaveCollision
  (params (A :type Object%20Object%20Reference))
  (bind _isplayer (|CallParentFunction A))
  (if _isplayer
    (Widget|RemovefromParent (Variables|Default|GetInteractionWidget))))