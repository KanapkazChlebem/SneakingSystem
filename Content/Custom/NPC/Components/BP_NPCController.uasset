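; AI controller for stealth NPCs that runs BT_NPC and reacts to the player and alerted allies through sight and hearing perception.
; Timers raise suspicion while a visible player crouches and lower it after losing sight, updating each NPC's HUD bar.
; Standing in view or maxed suspicion triggers the pawn's behavior: chase, chase while calling allies by noise, or flee.
; Results feed Blackboard keys that drive the tree.
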(event OnTargetPerceptionUpdated(AIPerception)
  (params (Actor :type Actor%20Object%20Reference) (Stimulus :type AI%20Stimulus%20Structure))
  (Variables|Default|SetCurrentStimulus Stimulus)
  (CallFunction|HandleSoundSense Actor)
  (CallFunction|HandleSightSense Actor))

(event EventBeginPlay
  (bind _asbp_hud (Utilities|Casting|CastToBP_HUD (HUD|GetHUD (Game|GetPlayerController 0)))
    (:then
      (Variables|Default|SetBPHUDRef _asbp_hud))
    (:CastFailed
      (Development|PrintString "oooof"))))

(event EventTick
  (params (DeltaSeconds :type Float%20%28single-precision%29)))

(event EventPossess
  (params (PossessedPawn :type Pawn%20Object%20Reference))
  (bind _output_get (Variables|Default|SetPossessed%20Pawn PossessedPawn))
  (AI|RunBehaviorTree "/Game/Custom/NPC/Behavior/Tree/BT_NPC.BT_NPC")
  (bind _behavior (Class|BPIBehavior|GetBehavior(Message) (Actor|GetComponentbyClass _output_get "/Game/Custom/NPC/Components/BP_SneakingComponent.BP_SneakingComponent_C")))
  (Variables|Default|SetBehavior _behavior)
  (bind _outactors (Actor|GetAllActorsOfClasswithTag "/Game/Custom/NPC/BP_NPCCharacter.BP_NPCCharacter_C" "NPC"))
  (bind (_array_element _array_index) (Utilities|Array|ForEachLoopwithBreak _outactors :!label _label)
    (:LoopBody
      (if (== _array_element (Variables|Default|GetPossessed%20Pawn))
        (Variables|Default|SetNPCID _array_index)
        (goto _label Break)))))

(fn ConstructionScript)

(fn SupressSuspicion
  (if (> (Variables|Default|GetSuspicionCounter) 0)
    (bind _returnvalue (Utilities|Time|SetTimerbyEvent (EventDispatchers|CreateEvent :!event ReduceSuspicion) 0.5 true))
    (Variables|Default|SetSuspisionSupressionTimer _returnvalue)))

(fn ReduceSuspicion
  (bind _suspicioncounter (Variables|Default|GetSuspicionCounter))
  (if (not (Variables|Default|GetisPlayerVisible))
    (if (> _suspicioncounter 0)
      (bind _result (Math|Integer|DecrementInt _suspicioncounter)
        (:%20%20
          (Default|UpdateSusBaronHud (Variables|Default|GetBPHUDRef) _result (Variables|Default|GetNPCID))))
      (else
        (Utilities|Time|ClearandInvalidateTimerbyHandle (Variables|Default|GetSuspisionSupressionTimer) :!label _label)
        (AI|Components|Blackboard|SetValueasBool (Variables|Default|GetBlackboard) (Variables|Default|GetIsSus) false)
        (AI|Components|Blackboard|SetValueasBool (Variables|Default|GetBlackboard) (Variables|Default|GetIsAfraid) false)))
    (else
      (goto _label))))

(fn IncrementSuspicion
  (if (Variables|Default|GetisPlayerVisible)
    (bind _result (Math|Integer|IncrementInt (Variables|Default|GetSuspicionCounter))
      (:%20%20
        (Default|UpdateSusBaronHud (Variables|Default|GetBPHUDRef) _result (Variables|Default|GetNPCID))))))

(fn HandleSoundSense
  (params (Actor :type Actor%20Object%20Reference))
  (bind _returnvalue (Class|AIPerceptionSystem|GetSenseClassforStimulus (Variables|Default|GetCurrentStimulus)))
  (if (== _returnvalue "/Script/AIModule.AISense_Hearing")
    (if (Actor|ActorHasTag Actor "Player") ; Is player?
      (AI|Components|Blackboard|SetValueasVector (Variables|Default|GetBlackboard) (Variables|Default|GetSoundLocation) (.StimulusLocation (Utilities|Struct|BreakAIStimulus (Variables|Default|GetCurrentStimulus))))
      (elif (Actor|ActorHasTag Actor "NPC") ; Is an NPC?
        (bind _asbp_npccontroller (Utilities|Casting|CastToBP_NPCController (AI|GetAIController Actor))
          (:then
            (if (Variables|BP_NPCController_C|GetIsAlerted _asbp_npccontroller) ; Heard NPC Notice Player
              (if (not (Variables|Default|GetisPlayerVisible)) ; Not alerted yet
                (Variables|Default|SetNPC Actor)
                (CallFunction|OnNPCHeard))))
          (:CastFailed
            (Development|PrintString "Wrong Controller!")))))))

(fn StartTimertoSupressSuspcion
  (Utilities|Time|SetTimerbyEvent (EventDispatchers|CreateEvent :!event SupressSuspicion) (Variables|Default|GetTimeToSupressSuspicion)))

(fn OnChaseBehavior
  (Variables|Default|SetIsAlerted true)
  (CallFunction|StartTimertoSupressSuspcion)
  (switch Utilities|FlowControl|Switch|SwitchonEBehavior (Variables|Default|GetBehavior)
    (:NewEnumerator0
      ;[1 1 1] Clear Timers and set actor to follow (Chase)
      (CallFunction|ClearTimers :!label _label)
      (CallFunction|AITreeFollowPlayer))
    (:NewEnumerator1
      (CallFunction|CallNPC)
      (goto _label))
    (:NewEnumerator3
      (CallFunction|RunAway)
      (CallFunction|ClearTimers)))
  (bind _output_get (Variables|Default|SetSuspicionCounter (Variables|Default|GetMaxSuspicion)))
  (Default|UpdateSusBaronHud (Variables|Default|GetBPHUDRef) _output_get (Variables|Default|GetNPCID)))

(fn IncreaseSuspicion
  (bind _blackboard (Variables|Default|GetBlackboard))
  ;[1 1 1] When player hides while not detected
  (bind _inhidingspot (Class|BPISneaking|IsHiding(Message) (Variables|Default|GetvisibleActor)))
  (if _inhidingspot
    (Utilities|Time|ClearandInvalidateTimerbyHandle (Variables|Default|GetSuspicionTimer))
    (CallFunction|StartTimertoSupressSuspcion)
    (else
      ;[1 1 1] When player stands up in view, begin chase
      (if (AI|Components|NavMovement|IsCrouching (Actor|GetComponentbyClass (Variables|Default|GetvisibleActor) "/Script/Engine.CharacterMovementComponent"))
        ;[1 1 1] Increase Suspicion when player is visibly sneaking
        (if (< (Variables|Default|GetSuspicionCounter) (Variables|Default|GetSuspicionTreshold))
          (CallFunction|IncrementSuspicion)
          (elif (< (Variables|Default|GetSuspicionCounter) (Variables|Default|GetMaxSuspicion))
            ;[1 1 1] Change NPC state to Suspicious
            (Development|PrintString "Hmm?")
            (CallFunction|IncrementSuspicion)
            (AI|Components|Blackboard|SetValueasVector _blackboard (Variables|Default|GetLastSeenLocation) (Transformation|GetActorLocation (Variables|Default|GetvisibleActor)))
            (AI|Components|Blackboard|SetValueasBool _blackboard (Variables|Default|GetIsSus) true)
            (else
              ;[1 1 1] Max Suspicion reached
              (Development|PrintString "I See you!")
              (CallFunction|OnChaseBehavior))))
        (else
          (Utilities|Time|ClearandInvalidateTimerbyHandle (Variables|Default|GetSuspicionTimer))
          (CallFunction|OnChaseBehavior))))))

(fn HandleSightSense
  (params (visibleActor :type Actor%20Object%20Reference))
  (bind _returnvalue (Class|AIPerceptionSystem|GetSenseClassforStimulus (Variables|Default|GetCurrentStimulus)))
  (if (== _returnvalue "/Script/AIModule.AISense_Sight")
    (bind _output_get (Variables|Default|SetvisibleActor visibleActor))
    (if (and (Actor|ActorHasTag _output_get "Player") (Utilities|Struct|BreakAIStimulus (Variables|Default|GetCurrentStimulus)))
      (bind _inhidingspot (Class|BPISneaking|IsHiding(Message) _output_get))
      (if (not _inhidingspot) ; If NPC notices Player Hidden, he doesn't react
        (Variables|Default|SetisPlayerVisible true) ; Can see Player
        (Utilities|Time|ClearandInvalidateTimerbyHandle (Variables|Default|GetTimerToLoseSight))
        (if (AI|Components|NavMovement|IsCrouching (Actor|GetComponentbyClass _output_get "/Script/Engine.CharacterMovementComponent")) ; Player is sneaking
          (bind _returnvalue_2 (Utilities|Time|SetTimerbyEvent (EventDispatchers|CreateEvent :!event IncreaseSuspicion) 0.5 true))
          (Variables|Default|SetSuspicionTimer _returnvalue_2)
          (else
            (CallFunction|OnChaseBehavior))))
      (elif (Actor|ActorHasTag _output_get "Player")
        (CallFunction|StartTimertoLoseSightOfPlayer)
        (if (AI|Components|NavMovement|IsCrouching (Actor|GetComponentbyClass _output_get "/Script/Engine.CharacterMovementComponent")) ; Player is sneaking
          ;[1 1 1] Reduce Suspicion to 0
          (CallFunction|ClearTimers)
          (CallFunction|SupressSuspicion)
          (elif (> (Variables|Default|GetSuspicionCounter) 0)
            ;[1 1 1] Stop following, move to last seen position
            (CallFunction|ClearTimers)
            (AI|Components|Blackboard|SetValueasVector (Variables|Default|GetBlackboard) (Variables|Default|GetLastSeenLocation) (Transformation|GetActorLocation (Variables|Default|GetvisibleActor)))
            (CallFunction|StartTimertoSupressSuspcion)
            (AI|Components|Blackboard|SetValueasObject (Variables|Default|GetBlackboard) (Variables|Default|GetPlayerActor) 0)
            (Development|PrintString "Stop Hiding!")))))))

(fn ClearTimers
  (Utilities|Time|ClearandInvalidateTimerbyHandle (Variables|Default|GetSuspicionTimer)))

(fn OnNPCHeard
  (Variables|Default|SetIsAlerted true)
  (switch Utilities|FlowControl|Switch|SwitchonEBehavior (Variables|Default|GetBehavior)
    (:NewEnumerator0
      (CallFunction|ClearTimers :!label _label)
      (CallFunction|AITreeFollowHeardNPCSound))
    (:NewEnumerator1
      (goto _label))
    (:NewEnumerator3
      (CallFunction|RunAway))))

(fn CallNPC
  (bind _possessed_pawn (Variables|Default|GetPossessed%20Pawn))
  (Class|AISenseHearing|ReportNoiseEvent (Transformation|GetActorLocation _possessed_pawn) 1.0 _possessed_pawn (Variables|Default|GetNPC%20Notify%20Range) "None"))

(fn RunAway
  (AI|Components|Blackboard|SetValueasBool (Variables|Default|GetBlackboard) (Variables|Default|GetIsAfraid) true))

(fn AITreeFollowHeardNPCSound
  (AI|Components|Blackboard|SetValueasVector (Variables|Default|GetBlackboard) (Variables|Default|GetAllySoundLocation) (Transformation|GetActorLocation (Variables|Default|GetNPC)))
  (if (Utilities|Struct|BreakAIStimulus (Variables|Default|GetCurrentStimulus)) ; Is Calling NPC visible?
    (AI|Components|Blackboard|SetValueasObject (Variables|Default|GetBlackboard) (Variables|Default|GetAlly) (Variables|Default|GetNPC))
    (else
      (CallFunction|StartTimertoSupressSuspcion))))

(fn AITreeFollowPlayer
  (bind _blackboard (Variables|Default|GetBlackboard))
  (AI|Components|Blackboard|SetValueasBool _blackboard (Variables|Default|GetHasLineOfSight) true)
  (AI|Components|Blackboard|SetValueasObject _blackboard (Variables|Default|GetPlayerActor) (Variables|Default|GetvisibleActor)))

(fn StartTimertoLoseSightOfPlayer
  (bind _returnvalue (Utilities|Time|SetTimerbyEvent (EventDispatchers|CreateEvent :!event LooseSightOfPlayer) (Variables|Default|GetTime%20to%20Loose%20Sight%20of%20Player)))
  (Variables|Default|SetTimerToLoseSight _returnvalue))

(fn LooseSightOfPlayer
  (Variables|Default|SetisPlayerVisible false) ; Can't see Player
  (AI|Components|Blackboard|SetValueasBool (Variables|Default|GetBlackboard) (Variables|Default|GetHasLineOfSight) false))