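; BP_SneakingComponent is an NPC component that stores a behavior value and launches its owning BP_NPCCharacter toward a destination in an arc.
; It caches the owner at BeginPlay, printing an error if the cast fails, and exposes the behavior through GetBehavior.
; JumptoDestination computes a projectile arc to the target raised by JumpHeight, then launches the character in Flying mode and restores Walking after a short fixed delay.
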(event EventBeginPlay
  (bind _asbp_npccharacter (Utilities|Casting|CastToBP_NPCCharacter (Components|GetOwner))
    (:then
      (Variables|Default|Setowner _asbp_npccharacter))
    (:CastFailed
      (Development|PrintString "Wrong Character!"))))

(event EventJumptoDestination
  (params (destination :type Vector :default "0, 0, 0"))
  (bind _owner (Variables|Default|Getowner))
  (bind _charactermovement (Variables|/Script/Engine.Character|GetCharacterMovement _owner))
  (bind _outlaunchvelocity (Game|SuggestProjectileVelocityCustomArc (Transformation|GetActorLocation (Variables|Default|Getowner)) (Math|Vector|MakeVector (.x destination) (.y destination) (+ (.z destination) (Variables|Default|GetJump%20Height))) 0.0 0.5))
  (Pawn|Components|CharacterMovement|SetMovementMode _charactermovement "MOVE_Flying" 0)
  (Character|LaunchCharacter _owner _outlaunchvelocity true true)
  (Utilities|FlowControl|Delay 0.4)
  (Pawn|Components|CharacterMovement|SetMovementMode _charactermovement "MOVE_Walking" 0))

(fn GetBehavior
  (return (Variables|Default|GetBehavior)))