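; AI controller for an NPC with stealth detection: it runs BT_NPC and turns perception stimuli into Blackboard values.
; Heard sounds set SoundLocation; seeing a standing player starts a chase immediately.
; A crouching player in view starts a looping timer for suspicion, which escalates to suspicious, then chase, and updates the HUD bar.
; Losing sight sets up timed suspicion decay, recording the last seen location if the player is standing.
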(event OnTargetPerceptionUpdated(AIPerception)
  (params (Actor :type Actor%20Object%20Reference) (Stimulus :type AI%20Stimulus%20Structure))
  (CallFunction|HandleSoundSense Stimulus)
  (CallFunction|HandleSightSense Actor Stimulus))

(event EventBeginPlay
  (bind _asbp_hud (Utilities|Casting|CastToBP_HUD (HUD|GetHUD (Game|GetPlayerController 0)))
    (:then
      (Variables|Default|SetBPHUDRef _asbp_hud))
    (:CastFailed
      (Development|PrintString "oooof"))))

(event EventTick
  (params (DeltaSeconds :type Float%20%28single-precision%29)))

(event EventPossess
  (params (PossessedPawn :type Pawn%20Object%20Reference))
  (AI|RunBehaviorTree "/Game/Custom/NPC/BT_NPC.BT_NPC"))

(fn ConstructionScript)

(fn SupressSuspicion
  (if (> (Variables|Default|GetSuspicionCounter) 0)
    (bind _returnvalue (Utilities|Time|SetTimerbyEvent (EventDispatchers|CreateEvent :!event ReduceSuspicion) 0.5 true))
    (Variables|Default|SetSuspisionSupressionTimer _returnvalue)))

(fn ReduceSuspicion
  (bind _suspicioncounter (Variables|Default|GetSuspicionCounter))
  (if (not (Variables|Default|GetisPlayerVisible))
    (if (> _suspicioncounter 0)
      (bind _result (Math|Integer|DecrementInt _suspicioncounter)
        (:%20%20
          (Default|UpdateSusBaronHud (Variables|Default|GetBPHUDRef) _result)))
      (else
        (Utilities|Time|ClearandInvalidateTimerbyHandle (Variables|Default|GetSuspisionSupressionTimer) :!label _label)
        (AI|Components|Blackboard|SetValueasBool (Variables|Default|GetBlackboard) (Variables|Default|GetIsSus) false)))
    (else
      (goto _label))))

(fn IncrementSuspicion
  (if (Variables|Default|GetisPlayerVisible)
    (bind _result (Math|Integer|IncrementInt (Variables|Default|GetSuspicionCounter))
      (:%20%20
        (Default|UpdateSusBaronHud (Variables|Default|GetBPHUDRef) _result)))))

(fn HandleSoundSense
  (params (Stimulus :type AI%20Stimulus%20Structure%20%28by%20ref%29))
  (bind _returnvalue (Class|AIPerceptionSystem|GetSenseClassforStimulus Stimulus))
  (if (== _returnvalue "/Script/AIModule.AISense_Hearing")
    (AI|Components|Blackboard|SetValueasVector (Variables|Default|GetBlackboard) (Variables|Default|GetSoundLocation) (.StimulusLocation (Utilities|Struct|BreakAIStimulus Stimulus)))))

(fn StartTimertoSupressSuspcion
  (CallFunction|SupressSuspicion))

(fn BeginChase
  (bind _blackboard (Variables|Default|GetBlackboard))
  ;[1 1 1] Clear Timer and set actor to follow
  (Utilities|Time|ClearandInvalidateTimerbyHandle (Variables|Default|GetSuspicionTimer))
  (Utilities|Time|ClearandInvalidateTimerbyHandle (Variables|Default|GetPlayerTimer))
  (AI|Components|Blackboard|SetValueasBool _blackboard (Variables|Default|GetHasLineOfSight) true)
  (AI|Components|Blackboard|SetValueasObject _blackboard (Variables|Default|GetPlayerActor) (Variables|Default|GetvisibleActor))
  (bind _output_get (Variables|Default|SetSuspicionCounter (Variables|Default|GetMaxSuspicion)))
  (Default|UpdateSusBaronHud (Variables|Default|GetBPHUDRef) _output_get))

(fn IncreaseSuspicion
  (bind _blackboard (Variables|Default|GetBlackboard))
  ;[1 1 1] When player stands up in view, begin chase
  (if (AI|Components|NavMovement|IsCrouching (Actor|GetComponentbyClass (Variables|Default|GetvisibleActor) "/Script/Engine.CharacterMovementComponent"))
    ;[1 1 1] Increase Suspicion when player is visibly sneaking
    (if (< (Variables|Default|GetSuspicionCounter) (Variables|Default|GetSuspicionTreshold))
      (CallFunction|IncrementSuspicion)
      (elif (< (Variables|Default|GetSuspicionCounter) (Variables|Default|GetMaxSuspicion))
        ;[1 1 1] Change NPC state to Suspicious
        (Development|PrintString "Hmm?")
        (CallFunction|IncrementSuspicion)
        (AI|Components|Blackboard|SetValueasVector _blackboard (Variables|Default|GetLastSeenLocation) (Transformation|GetActorLocation (Variables|Default|GetvisibleActor)))
        (AI|Components|Blackboard|SetValueasBool _blackboard (Variables|Default|GetIsSus) true)
        (else
          ;[1 1 1] Max Suspicion reached
          (Development|PrintString "I See you!")
          (CallFunction|BeginChase))))
    (else
      (Utilities|Time|ClearandInvalidateTimerbyHandle (Variables|Default|GetSuspicionTimer))
      (CallFunction|BeginChase))))

(fn HandleSightSense
  (params (visibleActor :type Actor%20Object%20Reference) (Stimulus :type AI%20Stimulus%20Structure%20%28by%20ref%29))
  (bind _blackboard (Variables|Default|GetBlackboard))
  (bind _returnvalue (Class|AIPerceptionSystem|GetSenseClassforStimulus Stimulus))
  (if (== _returnvalue "/Script/AIModule.AISense_Sight")
    (bind _output_get (Variables|Default|SetvisibleActor visibleActor))
    (if (and (Actor|ActorHasTag _output_get "Player") (Utilities|Struct|BreakAIStimulus Stimulus))
      (Variables|Default|SetisPlayerVisible true) ; Can see Player
      (if (AI|Components|NavMovement|IsCrouching (Actor|GetComponentbyClass _output_get "/Script/Engine.CharacterMovementComponent")) ; Player is sneaking
        (bind _returnvalue_2 (Utilities|Time|SetTimerbyEvent (EventDispatchers|CreateEvent :!event IncreaseSuspicion) 0.5 true))
        (Variables|Default|SetSuspicionTimer _returnvalue_2)
        (else
          (CallFunction|BeginChase)))
      (elif (Actor|ActorHasTag _output_get "Player")
        (Variables|Default|SetisPlayerVisible false) ; Can't see Player
        (if (AI|Components|NavMovement|IsCrouching (Actor|GetComponentbyClass _output_get "/Script/Engine.CharacterMovementComponent")) ; Player is sneaking
          ;[1 1 1] Reduce Suspicion to 0
          (Utilities|Time|ClearandInvalidateTimerbyHandle (Variables|Default|GetSuspicionTimer))
          (CallFunction|SupressSuspicion)
          (else
            ;[1 1 1] Stop following, move to last seen position
            (Utilities|Time|ClearandInvalidateTimerbyHandle (Variables|Default|GetSuspicionTimer))
            (AI|Components|Blackboard|SetValueasVector (Variables|Default|GetBlackboard) (Variables|Default|GetLastSeenLocation) (Transformation|GetActorLocation (Variables|Default|GetvisibleActor)))
            (Utilities|Time|SetTimerbyEvent (EventDispatchers|CreateEvent :!event StartTimertoSupressSuspcion) (Variables|Default|GetTimeToSupressSuspicion))
            (AI|Components|Blackboard|SetValueasBool _blackboard (Variables|Default|GetHasLineOfSight) false)
            (AI|Components|Blackboard|SetValueasObject _blackboard (Variables|Default|GetPlayerActor) 0)
            (Development|PrintString "Stop Hiding!")))))))