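; Player character component that handles stealth hiding, both in hiding-spot volumes and inside interactable objects.
; Hide/Unhide track occupied volumes in an array, so overlapping spots count as one hidden state.
; E enters BPI_HideInObject actors, moving the camera to their spring arm and disabling visibility, collision and movement; E with no overlaps restores them.
; Looping timers fade the camera's post-process weight, and IsHiding reports either state.
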(event EventHide
  (params (hidingSpotRef :type BP%20Hiding%20Spot%20Volume%20Object%20Reference))
  ;[1 1 1] Interaction with Hiding Spot Volume Objects
  (bind _returnvalue (Utilities|Array|Add (Variables|Default|GetHidingSpotVolRefs) hidingSpotRef))
  (if (== _returnvalue 0)
    (Variables|Default|SetisHiddenInVolume true)
    (CallFunction|InterpolatePostProcess)))

(event EventUnhide
  (params (hidingSpotRef :type BP%20Hiding%20Spot%20Volume%20Object%20Reference))
  (bind _hidingspotvolrefs (Variables|Default|GetHidingSpotVolRefs))
  ;[1 1 1] Interaction with Hiding Spot Volume Objects
  (if (Utilities|Array|IsEmpty _hidingspotvolrefs)
    (Development|PrintString "EmptyArray!") ; When Player leaves hiding volume in which he did not hide in (can hide only when crouched, can unhide anytime)
    (else
      (Utilities|Array|RemoveItem _hidingspotvolrefs hidingSpotRef)
      (if (Utilities|Array|IsEmpty _hidingspotvolrefs)
        (Variables|Default|SetisHiddenInVolume false)
        (CallFunction|ReverseInterpolatePostProcess)))))

(event EventBeginPlay
  (bind _asbp_third_person_character (Utilities|Casting|CastToBP_ThirdPersonCharacter (Components|GetOwner))
    (:then
      (Variables|Default|SetPlayerRef _asbp_third_person_character))
    (:CastFailed
      (Development|PrintString "Wrong character cast"))))

(event EventTick
  (params (DeltaSeconds :type Float%20%28single-precision%29)))

(event Input|KeyboardEvents|E
  (params (Key :type Key%20Structure :default "None"))
  (bind _playerref (Variables|Default|GetPlayerRef))
  (bind _playerref_2 (Variables|Default|GetPlayerRef))
  (bind _playerref_3 (Variables|Default|GetPlayerRef))
  (bind _playerref_4 (Variables|Default|GetPlayerRef))
  (bind _overlappingactors (Collision|GetOverlappingActors _playerref 0 :!class /Script/Engine.Actor))
  ;[1 1 1] Interaction With Hiding Spot Objects
  (:Pressed
    (if (Utilities|Array|IsEmpty _overlappingactors)
      (Class|BPIHideinObject|Interact(Message) (Variables|Default|GethidingSpotRef))
      (Variables|Default|SethidingSpotRef 0)
      (Transformation|AttachComponentToComponent (Variables|/Game/Custom/Character/BP_ThirdPersonCharacter.BP_ThirdPersonCharacter_C|GetFollowCamera _playerref_2) (Variables|/Game/Custom/Character/BP_ThirdPersonCharacter.BP_ThirdPersonCharacter_C|GetCameraBoom _playerref_2) (Variables|Default|GetSocket%20Name) "KeepRelative" "KeepRelative" "KeepRelative" true)
      (Rendering|SetActorHiddenInGame _playerref_3 false)
      (Collision|SetActorEnableCollision _playerref_3 true)
      (Variables|Default|SetisHiddenInObject false)
      (Pawn|Components|CharacterMovement|SetMovementMode (Variables|/Script/Engine.Character|GetCharacterMovement (Variables|Default|GetPlayerRef)) "MOVE_Walking" 0)
      (CallFunction|ReverseInterpolatePostProcess)
      (else
        (bind _array_element (Utilities|Array|ForEachLoopwithBreak _overlappingactors)
          (:LoopBody
            (if (Utilities|DoesObjectImplementInterface _array_element "/Game/Custom/HidingSpots/BPI_HideInObject.BPI_HideInObject_C")
              (bind _output_get (Variables|Default|SethidingSpotRef _array_element))
              (Class|BPIHideinObject|Interact(Message) _output_get)
              (if (not (Variables|Default|GetisHiddenInObject))
                (Transformation|AttachComponentToComponent (Variables|/Game/Custom/Character/BP_ThirdPersonCharacter.BP_ThirdPersonCharacter_C|GetFollowCamera (Variables|Default|GetPlayerRef)) (Utilities|Array|Get(acopy) (Actor|GetComponentsByClass _array_element "/Script/Engine.SpringArmComponent")) (Variables|Default|GetSocket%20Name) "KeepRelative" "KeepRelative" "KeepRelative" true)
                (Rendering|SetActorHiddenInGame _playerref_4 true)
                (Collision|SetActorEnableCollision _playerref_4 false)
                (Variables|Default|SetisHiddenInObject true)
                (Pawn|Components|CharacterMovement|DisableMovement (Variables|/Script/Engine.Character|GetCharacterMovement (Variables|Default|GetPlayerRef)))
                (CallFunction|InterpolatePostProcess)))))))))

(fn InterpolatePostProcess
  (Utilities|Time|ClearandInvalidateTimerbyHandle (Variables|Default|GetDecrementTimer))
  (bind _returnvalue (Utilities|Time|SetTimerbyEvent (EventDispatchers|CreateEvent :!event IncrementFloat) (Variables|Default|GetInterpolationPeriod) true))
  (Variables|Default|SetIncrementTimer _returnvalue))

(fn IncrementFloat
  (if (< (Variables|Default|GetInterpolatedValue) 1.0)
    (bind _output_get (Variables|Default|SetInterpolatedValue (+ (Variables|Default|GetInterpolatedValue) (Variables|Default|GetInterpolationPeriod))))
    (Class|CameraComponent|SetPostProcessBlendWeight (Variables|/Game/Custom/Character/BP_ThirdPersonCharacter.BP_ThirdPersonCharacter_C|GetFollowCamera (Variables|Default|GetPlayerRef)) _output_get)
    (else
      (Utilities|Time|ClearandInvalidateTimerbyHandle (Variables|Default|GetIncrementTimer)))))

(fn ReverseInterpolatePostProcess
  (Utilities|Time|ClearandInvalidateTimerbyHandle (Variables|Default|GetIncrementTimer))
  (bind _returnvalue (Utilities|Time|SetTimerbyEvent (EventDispatchers|CreateEvent :!event DecrementFloat) (Variables|Default|GetInterpolationPeriod) true))
  (Variables|Default|SetDecrementTimer _returnvalue))

(fn DecrementFloat
  (if (> (Variables|Default|GetInterpolatedValue) 0.0)
    (bind _output_get (Variables|Default|SetInterpolatedValue (- (Variables|Default|GetInterpolatedValue) (Variables|Default|GetInterpolationPeriod))))
    (Class|CameraComponent|SetPostProcessBlendWeight (Variables|/Game/Custom/Character/BP_ThirdPersonCharacter.BP_ThirdPersonCharacter_C|GetFollowCamera (Variables|Default|GetPlayerRef)) _output_get)
    (else
      (Utilities|Time|ClearandInvalidateTimerbyHandle (Variables|Default|GetDecrementTimer)))))

(fn IsHiding
  (return (or (Variables|Default|GetisHiddenInObject) (Variables|Default|GetisHiddenInVolume))))